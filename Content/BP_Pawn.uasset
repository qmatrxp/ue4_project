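; BP_Pawn is the player pawn in a ball-and-lives game, moved sideways along world Y by the MoveRight axis with sweep.
; On BeginPlay it creates the BPWidget UI and spawns a BP_Ball at its capsule if lives remain, binding the ball's BallDead and LiveDead dispatchers.
; Overlapping bonus pickups spawn another ball, remove a life or add a life, depending on type.
; A LiveDead function decrements lives while they are above zero.
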(event `InputAxis|MoveRight`
  (params (AxisValue :type "Float (single-precision)"))
  (`self.K2_AddActorWorldOffset` (`KismetMathLibrary.MakeVector` 0.0 AxisValue) true))

(event `self.ReceiveBeginPlay`
  (`self.SpawnBall`)
  (bind _returnvalue (`|CreateWidget` "/Game/Mesh/BPWidget.BPWidget_C"))
  (`UserWidget.AddToViewport` _returnvalue 0))

(event `self.ReceiveActorBeginOverlap`
  (params (OtherActor :type "Actor Object Reference"))
  (bind _live (`self.live`))
  (cast `/Game/BP_Bonus` OtherActor
    (:`then`
      (`self.SpawnBall`))
    (:`CastFailed`
      (cast `/Game/BP_Bonus_2` OtherActor
        (:`then`
          (if (`KismetMathLibrary.Conv_IntToBool` _live)
            (bind _result (`/Engine/EditorBlueprintResources/StandardMacros.DecrementInt` _live)
              (:`  `
                (set `self.live` _result)))))
        (:`CastFailed`
          (cast `/Game/BP_Bonus_3` OtherActor)
          (bind _result_2 (`/Engine/EditorBlueprintResources/StandardMacros.IncrementInt` (`self.live`))
            (:`  `
              (set `self.live` _result_2))))))))

(event `self.ReceiveTick`
  (params (DeltaSeconds :type "Float (single-precision)")))

(fn `LiveDead`
  (if (> (`self.live`) 0)
    (bind _result (`/Engine/EditorBlueprintResources/StandardMacros.DecrementInt` (`self.live`))
      (:`  `
        (set `self.live` _result)))))

(fn `SpawnBall`
  (if (not (<= (`self.live`) 0))
    (bind _returnvalue (`|SpawnActorFromClass` "/Game/BP_Ball.BP_Ball_C" (`SceneComponent.K2_GetComponentToWorld` (`self.Capsule`)) "Undefined" "OverrideRootScale" null null))
    (bind _output_get (set `self.BP_Ball` _returnvalue))
    (add `/Game/BP_Ball.Ball_Dead` _output_get (`|CreateDelegate` :!event `SpawnBall`))
    (add `/Game/BP_Ball.Live_Dead` _output_get (`|CreateDelegate` :!event `LiveDead`))))

(fn `UserConstructionScript`)