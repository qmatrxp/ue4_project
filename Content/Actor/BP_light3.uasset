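; BP_light3 is a spotlight actor that blinks a set number of times when play begins, then stays off.
; BeginPlay runs a latent loop that hides the SpotLight, waits TimeDisable, shows it, waits TimeEnable, then increments BlickCount.
; Once BlickCount reaches NumBlick, the loop exits and leaves the light hidden.
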(event `self.ReceiveBeginPlay`
  (if (< (`self.Blick_count`) (`self.Num_Blick`)) :!label _label
    (`SceneComponent.SetVisibility` (`self.SpotLight`) false false)
    (`KismetSystemLibrary.Delay` (`self.Time_Disable`))
    (`SceneComponent.SetVisibility` (`self.SpotLight`) true false)
    (`KismetSystemLibrary.Delay` (`self.Time_Enable`))
    (bind _result (`/Engine/EditorBlueprintResources/StandardMacros.IncrementInt` (`self.Blick_count`))
      (:`  `
        (set `self.Blick_count` _result)
        (goto _label)))
    (else
      (`SceneComponent.SetVisibility` (`self.SpotLight`) false false))))

(fn `UserConstructionScript`)