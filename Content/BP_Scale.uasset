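; BP_Scale is an actor that reduces its own scale when a BP_Ball overlaps it.
; On overlap, it calls the parent event, casts the other actor to BP_Ball, subtracts Scale from Scale3d and applies the result as the actor's 3D scale.
; A trailing two-second delay has nothing wired after it, and BeginPlay and Tick are unused.
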(event `self.ReceiveActorBeginOverlap`
  (params (OtherActor :type "Actor Object Reference"))
  (`parent.ReceiveActorBeginOverlap` OtherActor)
  (cast `/Game/BP_Ball` OtherActor)
  (bind _output_get (set `self.Scale_3d` (- (`self.Scale_3d`) (`self.scale`))))
  (`self.SetActorScale3D` _output_get)
  (`KismetSystemLibrary.Delay` 2.0))

(fn `UserConstructionScript`
  (`parent.UserConstructionScript`))