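; Brick-grid actor for a Breakout-style game, holding every block as a static mesh component.
; The construction script lays out an X by Y grid spaced by Padding, randomly choosing one of three AddStaticMeshComponent branches per cell.
; On BP_Ball hits, the material encodes toughness: one is indestructible, one swaps to a weaker material, others are destroyed.
; Destruction adds a BP_Pawn point and randomly may spawn one of four bonuses, the first also calling CallNewBall.
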(event `self.ReceiveHit`
  (params (MyComp :type "PrimitiveComponent Object Reference") (Other :type "Actor Object Reference") (OtherComp :type "PrimitiveComponent Object Reference") (bSelfMoved :type Boolean) (HitLocation :type "Vector Structure") (HitNormal :type "Vector Structure") (NormalImpulse :type "Vector Structure") (Hit :type "HitResult Structure (by ref)"))
  (bind _returnvalue (`KismetMathLibrary.MakeTransform` HitLocation (struct) (0.5 0.5 0.5)))
  (cast `/Game/BP_Ball` Other)
  (if (== (`PrimitiveComponent.GetMaterial` MyComp 0) "/Game/Texture/NewMaterial3.NewMaterial3")
    _
    (elif (== (`PrimitiveComponent.GetMaterial` MyComp 0) "/Game/Texture/NewMaterial.NewMaterial")
      (`PrimitiveComponent.SetMaterial` MyComp 0 "/Game/Texture/Material2.Material2")
      (else
        (`ActorComponent.K2_DestroyComponent` MyComp)
        (bind _asbp_pawn (cast `/Game/BP_Pawn` (`GameplayStatics.GetPlayerPawn` 0)))
        (bind _result (`/Engine/EditorBlueprintResources/StandardMacros.IncrementInt` (`/Game/BP_Pawn.Point` _asbp_pawn))
          (:`  `
            (set `/Game/BP_Pawn.Point` _result _asbp_pawn)
            (switch `int` (`KismetMathLibrary.RandomInteger` 6)
              (:`0`
                (`|SpawnActorFromClass` "/Game/BP_Bonus.BP_Bonus_C" _returnvalue "AlwaysSpawn" "OverrideRootScale" null null)
                (`self.New_Ball`))
              (:`1`
                (`|SpawnActorFromClass` "/Game/BP_Bonus_2.BP_Bonus_2_C" _returnvalue "AlwaysSpawn" "OverrideRootScale" null null))
              (:`2`
                (`|SpawnActorFromClass` "/Game/BP_Bonus_3.BP_Bonus_3_C" _returnvalue "AlwaysSpawn" "OverrideRootScale" null null))
              (:`3`
                (`|SpawnActorFromClass` "/Game/BP_Bonus_4.BP_Bonus_4_C" _returnvalue "AlwaysSpawn" "OverrideRootScale" null null)))))))))

(fn `UserConstructionScript`
  (bind _padding (`self.padding`))
  (for _index (range (+ (`self.x`) 1))
    (for _index_2 (range (+ (`self.y`) 1))
      (switch `int` (`KismetMathLibrary.RandomIntegerInRange` 0 5)
        (:`Default`
          (bind _returnvalue (`KismetMathLibrary.MakeTransform` (`KismetMathLibrary.MakeVector` (`KismetMathLibrary.Conv_IntToDouble` (* _index _padding)) (`KismetMathLibrary.Conv_IntToDouble` (* _index_2 _padding)))))
          (`AddComponent|NODE_AddStaticMeshComponent-2` :`RelativeTransform` _returnvalue))
        (:`0`
          (`AddComponent|NODE_AddStaticMeshComponent-0` :`RelativeTransform` _returnvalue))
        (:`1`
          (`AddComponent|NODE_AddStaticMeshComponent-3` :`RelativeTransform` _returnvalue))))))